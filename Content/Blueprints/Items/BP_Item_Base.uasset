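; BP_Item_Base is an item actor that the player picks up by clicking on it.
; On BeginPlay it caches the BP_PlayerCharacter pawn and binds its own OnClicked event.
; A click passes ItemData to that character through ReceiveItemData and destroys the actor, provided the cached reference is valid.
; GetIcon is an empty stub.
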(event `self.ReceiveBeginPlay`
  (`|ExecutionSequence`
    (:`then_0`
      (bind _asbp_player_character (cast `/Game/Blueprints/Player/BP_PlayerCharacter` (`GameplayStatics.GetPlayerPawn` 0)))
      (set `self.PlayerCharacter` _asbp_player_character))
    (:`then_1`
      (add `self.OnClicked` (delegate `OnClicked_Event`)))))

(event `OnClicked_Event` :!signature `self.OnClicked`
  (params (TouchedActor :type "Actor Object Reference") (ButtonPressed :type "Key Structure" :default "None"))
  (bind _playercharacter (`self.PlayerCharacter`)
    (:`then`
      (`/Game/Blueprints/Player/BP_PlayerCharacter.ReceiveItemData` _playercharacter (`self.ItemData`))
      (`self.K2_DestroyActor`))
    (:`else`)))

(fn `GetIcon`
  (returns (IconImage :type "Object Object Reference"))
  (return null))

(fn `UserConstructionScript`)