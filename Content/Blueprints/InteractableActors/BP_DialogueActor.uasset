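; BP_DialogueActor is a clickable world actor that supplies dialogue to the player.
; On BeginPlay it binds cursor-over, cursor-leave and click events, swapping the Cube mesh material to show hover state.
; A click casts the player pawn to BP_PlayerCharacter and passes the actor's Dialogues variable to its ReceiveDialogues function.
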(event `self.ReceiveBeginPlay`
  ; Changes material when hovered with the mouse
  (add `self.OnBeginCursorOver` (delegate `OnBeginCursorOver_Event`))
  (add `self.OnEndCursorOver` (delegate `OnEndCursorOver_Event`))
  ; When clicked, send dialogs to the player character
  (add `self.OnClicked` (delegate `OnClicked_Event`)))

(event `OnBeginCursorOver_Event` :!signature `self.OnBeginCursorOver`
  (params (TouchedActor :type "Actor Object Reference"))
  ; Changes material when hovered with the mouse
  (`PrimitiveComponent.SetMaterial` (`self.Cube`) 0 "/Game/StarterContent/Materials/M_AssetPlatform.M_AssetPlatform"))

(event `OnEndCursorOver_Event` :!signature `self.OnEndCursorOver`
  (params (TouchedActor :type "Actor Object Reference"))
  ; Changes material when hovered with the mouse
  (`PrimitiveComponent.SetMaterial` (`self.Cube`) 0 "/Game/LevelPrototyping/Materials/MI_Solid_Blue.MI_Solid_Blue"))

(event `OnClicked_Event` :!signature `self.OnClicked`
  (params (TouchedActor :type "Actor Object Reference") (ButtonPressed :type "Key Structure" :default "None"))
  ; When clicked, send dialogs to the player character
  (bind _asbp_player_character (cast `/Game/Blueprints/Player/BP_PlayerCharacter` (`GameplayStatics.GetPlayerPawn` 0)))
  (`/Game/Blueprints/Player/BP_PlayerCharacter.ReceiveDialogues` _asbp_player_character (`self.Dialogues`)))

(fn `UserConstructionScript`)